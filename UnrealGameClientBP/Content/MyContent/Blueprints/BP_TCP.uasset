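; BP_TCP is a TCP client test actor that connects to a configured IPv4 address and port on BeginPlay.
; Connection callbacks store the socket ID and show colored status on a TextRender, while received messages print to screen.
; Overlapping its StaticMesh sends a UTF-8 "Helloworld!", clearing the ID if sending fails.
; A TCPConnect retry function exists, but its looping-timer setup is unwired, so reconnection never runs.
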(event `self.ReceiveBeginPlay`
  (`self.Connect` (`self.ServerIPv4Address`) (`self.ServerPort`) (`|CreateDelegate` :!event `BP_TCP_AutoGenFunc`) (delegate `OnTCPConnected`) (delegate `OnTCPRecv`)))

(event `OnTCPDisconnected`
  (params (ConnectionId :type Integer))
  (bind _output_get (set `self.ServerSocketID` 0))
  (`self.SetTextMessage` "DisConnected" (make `Color` 0 0 255 255))
  (`KismetSystemLibrary.PrintString` (`KismetStringLibrary.Concat_StrStr` "[Disconnected]" "ConnectionID : " (`KismetStringLibrary.Conv_IntToString` _output_get))))

(event `OnTCPConnected`
  (params (ConnectionId :type Integer))
  (bind _output_get (set `self.ServerSocketID` ConnectionId))
  (`self.SetTextMessage` "Connected" (make `Color` 0 255 0 255))
  (`KismetSystemLibrary.PrintString` (`KismetStringLibrary.Concat_StrStr` "[Connected]" "ConnectionID : " (`KismetStringLibrary.Conv_IntToString` _output_get))))

(event `OnTCPRecv`
  (params (ConnectionId :type Integer) (Message :type "Array of Byte (by ref)"))
  (bind _returnvalue (`self.Message_ReadString` Message (`KismetArrayLibrary.Array_Length` Message)))
  (`KismetSystemLibrary.PrintString` _returnvalue))

(event `self.StaticMesh.OnComponentBeginOverlap`
  (params (OverlappedComponent :type "PrimitiveComponent Object Reference") (OtherActor :type "Actor Object Reference") (OtherComp :type "PrimitiveComponent Object Reference") (OtherBodyIndex :type Integer) (bFromSweep :type Boolean) (SweepResult :type "HitResult Structure (by ref)"))
  (bind _bsuccess (`self.SendMessage_UTF8String` "Helloworld!"))
  (if (not _bsuccess)
    (set `self.ServerSocketID` 0)))

(fn `BP_TCP_AutoGenFunc`
  (params (ConnectionId :type Integer)))

(fn `BP_TCP_AutoGenFunc1`
  (params (ConnectionId :type Integer) (Message :type "Array of Byte (by ref)"))
  (return))

(fn `BP_TCP_AutoGenFunc2`
  (params (ConnectionId :type Integer)))

(fn `BP_TCP_AutoGenFunc3`
  (params (ConnectionId :type Integer)))

(fn `SendMessage_UTF8String`
  (params (UTF8String :type String))
  (returns (bSuccess :type Boolean))
  (bind _returnvalue (`self.SendData` (`self.ServerSocketID`) (`self.Conv_StringToBytes` UTF8String)))
  (return _returnvalue))

(fn `SetTextMessage`
  (params (Text :type String) (TextColor :type "Color Structure"))
  (bind _textrender (`self.TextRender`))
  (`TextRenderComponent.K2_SetText` _textrender (`KismetTextLibrary.Conv_StringToText` Text))
  (`TextRenderComponent.SetTextRenderColor` _textrender TextColor))

(fn `TCPConnect`
  (if (not (`self.bTCPConnected`))
    (`self.Connect` (`self.ServerIPv4Address`) (`self.ServerPort`) (`|CreateDelegate` :!event `BP_TCP_AutoGenFunc3`) (`|CreateDelegate` :!event `BP_TCP_AutoGenFunc2`) (`|CreateDelegate` :!event `BP_TCP_AutoGenFunc1`))))

(fn `UserConstructionScript`)